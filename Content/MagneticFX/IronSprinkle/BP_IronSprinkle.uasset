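; Iron filings shaker actor that sprinkles Niagara particles onto a BP_Card when tipped over.
; Tick activates the emitter while the actor's up vector tilts over 60 degrees from vertical, otherwise deactivates it.
; The Niagara export callback adds frame time for each particle within 50 units of the card in 2D.
; Once that total passes two, it swaps the card's plane to a spread-filings material and latches IsSprinkled.
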(event EventBeginPlay
  (Niagara|SetNiagaraVariable(Object) (Variables|Default|GetNiagara) "BPCallbackHandler" self)
  (bind _returnvalue (Actor|GetActorOfClass "/Game/MagneticFX/IronSprinkle/BP_Card.BP_Card_C"))
  (Variables|Default|SetCard _returnvalue))

(event Collision|EventActorBeginOverlap
  (params (OtherActor :type Actor%20Object%20Reference)))

(event EventTick
  (params (DeltaSeconds :type Float%20%28single-precision%29))
  (bind _niagara (Variables|Default|GetNiagara))
  (if (< (Math|Vector|DotProduct (Transformation|GetActorUpVector) (Math|Vector|VectorUp)) 0.5)
    (Components|Activation|Activate _niagara false)
    (else
      (Components|Activation|Deactivate _niagara))))

(event EventParticleData
  (params (Data :type Array%20of%20Basic%20Particle%20Data%20Structures) (NiagaraSystem :type Niagara%20System%20Object%20Reference) (SimulationPositionOffset :type Vector%20%28by%20ref%29 :default "0, 0, 0"))
  (if (not (Variables|Default|GetisSprinkled))
    (for _array_element Data
      (if (<= (Math|Vector|Distance2D(Vector) (.Position (Utilities|Struct|BreakBasicParticleData _array_element)) (Transformation|GetActorLocation (Variables|Default|GetCard))) 5e+01)
        (bind _output_get (Variables|Default|SetElapsedTime (+ (Variables|Default|GetElapsedTime) (Utilities|Time|GetWorldDeltaSeconds))))
        (if (> _output_get 2.0)
          (Rendering|Material|SetMaterial (Variables|/Game/MagneticFX/IronSprinkle/BP_Card.BP_Card_C|GetPlane (Variables|Default|GetCard)) 0 "/Game/Scene2/materials/IronFillingSpread.IronFillingSpread")
          (Development|PrintString "Hello")
          (Variables|Default|SetisSprinkled true))))))

(fn ConstructionScript)