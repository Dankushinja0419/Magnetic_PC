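; BP_Card is the card actor in the IronSprinkle magnetism effect, revealing iron filings once it rests on a magnet and has been sprinkled.
; Overlaps with actors tagged Magnets toggle an OnMagnet flag and print it.
; Tick checks that flag and IsSprinkled on the BP_IronSprinkle found at BeginPlay, then after a one-second delay swaps the plane to the IronFillingDecal material and latches Magnetised.
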(event EventBeginPlay
  (bind _returnvalue (Actor|GetActorOfClass "/Game/MagneticFX/IronSprinkle/BP_IronSprinkle.BP_IronSprinkle_C"))
  (Variables|Default|SetIronSprinkle _returnvalue))

(event Collision|EventActorBeginOverlap
  (params (OtherActor :type Actor%20Object%20Reference))
  (if (Actor|ActorHasTag OtherActor "Magnets")
    (Variables|Default|SetOnMagnet true)
    (Development|PrintString (Utilities|String|ToString(Boolean) (Variables|Default|GetOnMagnet)))))

(event EventTick
  (params (DeltaSeconds :type Float%20%28single-precision%29))
  (if (not (Variables|Default|GetMagnetised))
    (if (and (Variables|Default|GetOnMagnet) (Variables|/Game/MagneticFX/IronSprinkle/BP_IronSprinkle.BP_IronSprinkle_C|GetisSprinkled (Variables|Default|GetIronSprinkle)))
      (Utilities|FlowControl|Delay 1.0)
      (Rendering|Material|SetMaterial (Variables|Default|GetPlane) 0 "/Game/JaredStuff/materials/IronFillingDecal.IronFillingDecal")
      (Variables|Default|SetMagnetised true))))

(event Collision|EventActorEndOverlap
  (params (OtherActor :type Actor%20Object%20Reference))
  (if (Actor|ActorHasTag OtherActor "Magnets")
    (Variables|Default|SetOnMagnet false)
    (Development|PrintString (Utilities|String|ToString(Boolean) (Variables|Default|GetOnMagnet)))))

(fn ConstructionScript)