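; BP_ChargedParticle is a particle actor in MagneticFX whose appearance shows the sign of its charge.
; UpdateColor sets the cube's material to metallic blue for positive Charge, red for negative and burnished steel for zero.
; BeginPlay applies a dynamic material, which UpdateColor immediately replaces.
; Tick billboards the whole actor toward the cached player camera manager's location; DisplayCharge is an empty stub.
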(event Custom|UpdateColor
  (bind _charge (Variables|Default|GetCharge))
  (if (> _charge 0.0)
    (Rendering|Material|SetMaterial (Variables|Default|GetCube) 0 "/Game/JaredStuff/materials/MetallicBlueColour.MetallicBlueColour")
    (elif (< _charge 0.0)
      (Rendering|Material|SetMaterial (Variables|Default|GetCube) 0 "/Game/JaredStuff/materials/MetallicRedColour.MetallicRedColour")
      (else
        (Rendering|Material|SetMaterial (Variables|Default|GetCube) 0 "/Game/StarterContent/Materials/M_Metal_Burnished_Steel.M_Metal_Burnished_Steel")))))

(event Custom|DisplayCharge)

(event EventBeginPlay
  (bind _returnvalue (Actor|GetActorOfClass "/Script/Engine.PlayerCameraManager"))
  (Variables|Default|SetHeadCamera _returnvalue)
  (bind _returnvalue_2 (Rendering|Material|CreateDynamicMaterialInstance 0 "None" "None" :!class /Script/Engine.KismetMaterialLibrary))
  (bind _output_get (Variables|Default|SetDynamicMaterial _returnvalue_2))
  (Rendering|Material|SetMaterial (Variables|Default|GetCube) 0 _output_get)
  (CallFunction|UpdateColor))

(event Collision|EventActorBeginOverlap
  (params (OtherActor :type Actor%20Object%20Reference)))

(event EventTick
  (params (DeltaSeconds :type Float%20%28single-precision%29))
  (Transformation|SetActorRotation (Math|Rotator|MakeRotfromX (- (Camera|GetCameraLocation (Variables|Default|GetHeadCamera)) (Transformation|GetActorLocation)))))

(fn ConstructionScript)