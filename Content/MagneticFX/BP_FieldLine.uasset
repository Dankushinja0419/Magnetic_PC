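; Field line actor that traces and draws one electric field line from a start location when GenerateFieldLine runs.
; It steps a fixed distance along FieldManager's normalized field vector, adding spline points until strength falls below a minimum or steps run out.
; Each spline segment becomes a cylinder spline mesh with a dynamic arrow material, colored through a curve by the sampled field strength.
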(event EventBeginPlay)

(event Collision|EventActorBeginOverlap
  (params (OtherActor :type Actor%20Object%20Reference)))

(event EventTick
  (params (DeltaSeconds :type Float%20%28single-precision%29)))

(fn ConstructionScript)

(fn GenerateFieldLine
  (bind _spline (Variables|Default|GetSpline))
  (bind _startlocation (Variables|Default|GetStartLocation))
  (bind _spline_2 (Variables|Default|GetSpline))
  (bind _spline_3 (Variables|Default|GetSpline))
  (for _array_element (Variables|Default|GetSplineMeshes)
    (if (Utilities|IsValid _array_element)
      (Components|DestroyComponent _array_element)))
  (Spline|ClearSplinePoints _spline true)
  (Spline|AddSplinePoint _spline _startlocation "World" true)
  (bind _output_get (LocalVariables|SetCurrentPosition _startlocation))
  (for _index (range 0 (- (Variables|Default|GetMaxSteps) 1))
    (bind _finalelectricfield (Default|GetElectricFieldVector (Variables|Default|GetFieldManager) _output_get))
    (bind _output_get_2 (LocalVariables|SetStrength (Math|Vector|VectorLength _finalelectricfield)))
    (Utilities|Array|Add (Variables|Default|GetStrengthArray) _output_get_2)
    (if (not (< _output_get_2 (Variables|Default|GetMinFieldStrength)))
      (bind _output_get_3 (LocalVariables|SetNextPosition (+ (LocalVariables|GetCurrentPosition) (* (Variables|Default|GetStepSize) (Math|Vector|Normalize _finalelectricfield)))))
      (Spline|AddSplinePoint (Variables|Default|GetSpline) _output_get_3 "World" true)
      (LocalVariables|SetCurrentPosition _output_get_3)))
  (Spline|UpdateSpline _spline_3)
  (bind _output_get_4 (LocalVariables|SetNumsOfSpline (Spline|GetNumberOfSplinePoints _spline_3)))
  (for _index_2 (range 0 (- _output_get_4 2))
    (bind _returnvalue (AddComponent|AddSplineMeshComponent true))
    (Utilities|Array|Add (Variables|Default|GetSplineMeshes) _returnvalue)
    (Transformation|SetMobility _returnvalue "Movable")
    (Components|StaticMesh|SetStaticMesh _returnvalue "/Engine/VREditor/FloatingText/LineSegmentCylinder.LineSegmentCylinder")
    (SplineMesh|SetStartandEnd _returnvalue (.Location (Spline|GetLocationandTangentatSplinePoint _spline_2 _index_2 "World")) (.Tangent (Spline|GetLocationandTangentatSplinePoint _spline_2 _index_2 "World")) (.Location (Spline|GetLocationandTangentatSplinePoint _spline_2 (+ _index_2 1) "World")) (.Tangent (Spline|GetLocationandTangentatSplinePoint _spline_2 (+ _index_2 1) "World")) true :!class /Script/Engine.SplineMeshComponent)
    (SplineMesh|SetEndScale _returnvalue "(X=3.000000,Y=3.000000)" true :!class /Script/Engine.SplineMeshComponent)
    (SplineMesh|SetStartScale _returnvalue "(X=3.000000,Y=3.000000)" true :!class /Script/Engine.SplineMeshComponent)
    (bind _returnvalue_2 (Rendering|Material|CreateDynamicMaterialInstance "/Game/MagneticFX/Arrow/ArrowMat.ArrowMat" "None" "None" :!class /Script/Engine.KismetMaterialLibrary))
    (Rendering|Material|SetMaterial _returnvalue 0 _returnvalue_2)
    (Rendering|Material|SetVectorParameterValue _returnvalue_2 "Color" (Class|CurveLinearColor|GetClampedLinearColorValue (Variables|Default|GetColorCurve) (/ (Utilities|Array|Get(acopy) (Variables|Default|GetStrengthArray) _index_2) 45.0)) :!class /Script/Engine.MaterialInstanceDynamic)))