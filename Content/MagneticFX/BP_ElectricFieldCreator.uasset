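; Actor that visualizes the electric field of the level's BP_ChargedParticle actors with a 3D grid of arrows.
; BeginPlay caches the charges and spawns BP_FieldArrow actors from its starting location.
; Each tick sums scaled inverse-square contributions per axis at every arrow, skipping very close charges, and points arrows along the normalized field.
; Clamped strength updates running min/max values; arrows setting a new extreme skip rotation that tick.
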(event Custom|CreateField
  (bind _gridspacing (Variables|Default|GetGridSpacing))
  (for _index (range 0 (- (Variables|Default|GetX_Length) 1))
    (for _index_2 (range 0 (- (Variables|Default|GetY_Length) 1))
      (for _index_3 (range 0 (- (Variables|Default|GetZ_Length) 1))
        (bind _output_get (Variables|Default|SetArrowLocation (+ (Variables|Default|GetInitialPosition) (Math|Vector|MakeVector (* _index _gridspacing) (* _index_2 _gridspacing) (* _index_3 _gridspacing)))))
        (bind _returnvalue (Game|SpawnActorfromClass "/Game/MagneticFX/BP_FieldArrow.BP_FieldArrow_C" (Math|Conversions|ToTransform(Vector) _output_get) "Undefined" "MultiplyWithRoot" 0 0))
        (Transformation|SetActorLocation _returnvalue _output_get false false)
        (Utilities|Array|Add (Variables|Default|GetArrowArray) _returnvalue)))))

(event Custom|UpdateArrowVector
  (for _array_element (Variables|Default|GetArrowArray)
    (bind _result (CallFunction|GetElectricFieldComponent "X" (Transformation|GetActorLocation _array_element) (Variables|Default|GetMagneticScale)))
    (Variables|Default|SeteX _result)
    (bind _result_2 (CallFunction|GetElectricFieldComponent "Y" (Transformation|GetActorLocation _array_element) (Variables|Default|GetMagneticScale)))
    (Variables|Default|SeteY _result_2)
    (bind _result_3 (CallFunction|GetElectricFieldComponent "Z" (Transformation|GetActorLocation _array_element) (Variables|Default|GetMagneticScale)))
    (Variables|Default|SeteZ _result_3)
    (Variables|Default|SetFieldStrength (Math|Float|Clamp(Float) (+ (Math|Float|Absolute(Float) (Variables|Default|GeteX)) (Math|Float|Absolute(Float) (Variables|Default|GeteY)) (Math|Float|Absolute(Float) (Variables|Default|GeteZ))) 0.02 2.0))
    (if (< (Variables|Default|GetFieldStrength) (Variables|Default|GetMinFieldStrength))
      (Variables|Default|SetMinFieldStrength (Variables|Default|GetFieldStrength))
      (elif (> (Variables|Default|GetFieldStrength) (Variables|Default|GetMaxFieldStrength))
        (Variables|Default|SetMaxFieldStrength (Variables|Default|GetFieldStrength))
        (else
          (Transformation|SetActorRotation _array_element (Math|Rotator|MakeRotfromX (Math|Vector|Normalize (Math|Vector|MakeVector (Variables|Default|GeteX) (Variables|Default|GeteY) (Variables|Default|GeteZ))))))))))

(event EventBeginPlay
  (Variables|Default|SetInitialPosition (Transformation|GetActorLocation))
  (bind _outactors (Actor|GetAllActorsOfClass "/Game/MagneticFX/BP_ChargedParticle.BP_ChargedParticle_C"))
  (Variables|Default|SetChargeArray _outactors)
  (CallFunction|CreateField))

(event Collision|EventActorBeginOverlap
  (params (OtherActor :type Actor%20Object%20Reference)))

(event EventTick
  (params (DeltaSeconds :type Float%20%28single-precision%29))
  (CallFunction|UpdateArrowVector))

(fn ConstructionScript)

(fn GetElectricFieldComponent
  (params (Direction :type EAxis%20Enum :default "None") (ArrowPosition :type Vector) (MagneticScale :type Float%20%28double-precision%29))
  (LocalVariables|SetArrowLocation ArrowPosition)
  (for _array_element (Variables|Default|GetChargeArray)
    (LocalVariables|SetVectorLength (Math|Vector|VectorLength (- ArrowPosition (Transformation|GetActorLocation _array_element))))
    (LocalVariables|SetCharge (Variables|/Game/MagneticFX/BP_ChargedParticle.BP_ChargedParticle_C|GetCharge _array_element))
    (if (not (< (Math|Vector|VectorLength (- ArrowPosition (Transformation|GetActorLocation _array_element))) 1.0))
      (switch Utilities|FlowControl|Switch|SwitchonEAxis Direction
        (:X
          (LocalVariables|SetarrowPositionComponent (.x (LocalVariables|GetArrowLocation)))
          (LocalVariables|SetchargePositionComponent (.x (Transformation|GetActorLocation _array_element))))
        (:Y
          (LocalVariables|SetarrowPositionComponent (.y (LocalVariables|GetArrowLocation)))
          (LocalVariables|SetchargePositionComponent (.y (Transformation|GetActorLocation _array_element))))
        (:Z
          (LocalVariables|SetarrowPositionComponent (.z (LocalVariables|GetArrowLocation)))
          (LocalVariables|SetchargePositionComponent (.z (Transformation|GetActorLocation _array_element)))))
      (LocalVariables|SeteSum (+ (LocalVariables|GeteSum) (* (/ (* (LocalVariables|GetCharge) (- (LocalVariables|GetarrowPositionComponent) (LocalVariables|GetchargePositionComponent))) (Math|Float|Power (LocalVariables|GetVectorLength) 3.0)) MagneticScale)))))
  (return (LocalVariables|GeteSum)))