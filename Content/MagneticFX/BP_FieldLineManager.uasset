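; Manager actor that creates and refreshes electric field lines for the charged particles in the level.
; On BeginPlay it gathers all BP_ChargedParticle actors and spawns one BP_FieldLine per positive charge, starting fractionally offset from its Cube.
; UpdateSpline moves those starts to the current charge positions and regenerates the lines.
; GetElectricFieldVector sums scaled inverse-square contributions from all charges, clamping distance to MinRadius.
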(event Custom|UpdateSpline
  (for (_array_element _array_index) (Variables|Default|GetPositiveCharges)
    (Variables|/Game/MagneticFX/BP_FieldLine.BP_FieldLine_C|SetStartLocation (Utilities|Array|Get(acopy) (Variables|Default|GetFieldLines) _array_index) (* (Transformation|GetWorldLocation (Variables|/Game/MagneticFX/BP_ChargedParticle.BP_ChargedParticle_C|GetCube _array_element)) 0.999999))
    (Default|GenerateFieldLine (Utilities|Array|Get(acopy) (Variables|Default|GetFieldLines) _array_index))))

(event EventBeginPlay
  (bind _outactors (Actor|GetAllActorsOfClass "/Game/MagneticFX/BP_ChargedParticle.BP_ChargedParticle_C"))
  (bind _output_get (Variables|Default|SetCharges _outactors))
  (for _array_element _output_get
    (if (> (Variables|/Game/MagneticFX/BP_ChargedParticle.BP_ChargedParticle_C|GetCharge _array_element) 0.0)
      (Utilities|Array|Add (Variables|Default|GetPositiveCharges) _array_element)
      (bind _returnvalue (Game|SpawnActorfromClass "/Game/MagneticFX/BP_FieldLine.BP_FieldLine_C" (Math|Conversions|ToTransform(Vector) (Transformation|GetWorldLocation (Variables|/Game/MagneticFX/BP_ChargedParticle.BP_ChargedParticle_C|GetCube _array_element))) "AlwaysSpawn" "MultiplyWithRoot" 0 0))
      (Utilities|Array|Add (Variables|Default|GetFieldLines) _returnvalue)
      (Variables|/Game/MagneticFX/BP_FieldLine.BP_FieldLine_C|SetStartLocation _returnvalue (* (Transformation|GetWorldLocation (Variables|/Game/MagneticFX/BP_ChargedParticle.BP_ChargedParticle_C|GetCube _array_element)) 0.999999))
      (Variables|/Game/MagneticFX/BP_FieldLine.BP_FieldLine_C|SetFieldManager _returnvalue self)
      (Default|GenerateFieldLine _returnvalue))))

(event Collision|EventActorBeginOverlap
  (params (OtherActor :type Actor%20Object%20Reference)))

(event EventTick
  (params (DeltaSeconds :type Float%20%28single-precision%29)))

(fn ConstructionScript)

(fn GetElectricFieldVector
  (params (WorldPosition :type Vector))
  (for _array_element (Variables|Default|GetCharges)
    (LocalVariables|SetChargesValue (Variables|/Game/MagneticFX/BP_ChargedParticle.BP_ChargedParticle_C|GetCharge _array_element))
    (bind _output_get (LocalVariables|SetR (- WorldPosition (Transformation|GetActorLocation _array_element))))
    (bind _output_get_2 (LocalVariables|SetStrength (/ (LocalVariables|GetChargesValue) (Math|Float|Power (Math|Float|Max(Float) (Math|Vector|VectorLength _output_get) (LocalVariables|GetMinRadius)) 2.0))))
    (LocalVariables|SetElectricField (+ (* _output_get_2 (Class|KismetMathLibrary|VectorNormalUnsafe _output_get) 50) (LocalVariables|GetElectricField))))
  (return (LocalVariables|GetElectricField)))