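; BP_VideoActivation is a trigger actor in the 360 folder that shows an interaction prompt while another actor overlaps it.
; On BeginPlay it creates an InteractUI widget for the first player controller, adds it to the viewport and hides it.
; Begin and end overlap events toggle that widget between visible and hidden, with no filtering on which actor overlaps.
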(event EventBeginPlay
  (bind _returnvalue (UserInterface|CreateWidget "/Game/360/InteractUI.InteractUI_C" (Game|GetPlayerController 0)))
  (bind _output_get (Variables|Default|SetUI _returnvalue))
  (UserInterface|Viewport|AddtoViewport _output_get 0)
  (Widget|SetVisibility (Variables|Default|GetUI) "Hidden"))

(event Collision|EventActorBeginOverlap
  (params (OtherActor :type Actor%20Object%20Reference))
  (Widget|SetVisibility (Variables|Default|GetUI) "Visible"))

(event EventTick
  (params (DeltaSeconds :type Float%20%28single-precision%29)))

(event Collision|EventActorEndOverlap
  (params (OtherActor :type Actor%20Object%20Reference))
  (Widget|SetVisibility (Variables|Default|GetUI) "Hidden"))

(fn ConstructionScript)