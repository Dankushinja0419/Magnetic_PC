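; Actor that plays a selected 360-degree video on a sphere in place of the surrounding level.
; StartVideo hides StaticMeshActors tagged "Surrounding", shows the sphere and plays the indexed source; open, play and end-event binding repeat inside the hide loop.
; At video end, ResetLevel restores the surroundings, BP_VideoActivation actors and the UI of the one overlapping the first-person character, then hides the sphere and closes the player.
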(event Custom|StartVideo
  (bind _video_player (Variables|Default|GetVideo%20Player))
  (bind _outactors (Actor|GetAllActorsOfClasswithTag "/Script/Engine.StaticMeshActor" "Surrounding"))
  (bind _output_get (Variables|Default|SetSurrounding _outactors))
  (for _array_element _output_get
    (Rendering|SetActorHiddenInGame _array_element true)
    (Media|MediaPlayer|OpenSource _video_player (Utilities|Array|Get(acopy) (Variables|Default|GetVideos) (Variables|Default|GetVideo%20Index)))
    (Media|MediaPlayer|Play _video_player :!class /Script/MediaAssets.MediaPlayer)
    (Rendering|SetActorHiddenInGame (Variables|Default|Get360Sphere) false)
    (Media|MediaPlayer|BindEventtoOnEndReached _video_player (delegate Custom|ResetLevel))))

(event Custom|ResetLevel
  (bind _returnvalue (Actor|GetActorOfClass "/Game/FirstPerson/Blueprints/BP_FirstPersonCharacter.BP_FirstPersonCharacter_C"))
  (Widget|SetVisibility (Variables|/Game/360/BP_VideoActivation.BP_VideoActivation_C|GetUI (Utilities|Array|Get(acopy) (Collision|GetOverlappingActors _returnvalue "/Game/360/BP_VideoActivation.BP_VideoActivation_C" :!class /Script/Engine.Actor))) "Visible")
  (for _array_element (Variables|Default|GetSurrounding)
    (Rendering|SetActorHiddenInGame _array_element false)
    (Rendering|SetActorHiddenInGame (Variables|Default|Get360Sphere) true)
    (bind _outactors (Actor|GetAllActorsOfClass "/Game/360/BP_VideoActivation.BP_VideoActivation_C"))
    (for _array_element_2 _outactors
      (Rendering|SetActorHiddenInGame _array_element_2 false)
      (Media|MediaPlayer|Close (Variables|Default|GetVideo%20Player) :!class /Script/MediaAssets.MediaPlayer))))

(event EventBeginPlay
  (Rendering|SetActorHiddenInGame (Variables|Default|Get360Sphere) true)
  (Media|MediaPlayer|Close (Variables|Default|GetVideo%20Player) :!class /Script/MediaAssets.MediaPlayer))

(fn ConstructionScript)