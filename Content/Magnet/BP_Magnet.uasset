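; BP_Magnet is an actor that lays out an elliptical ring of magnetic field points when play begins.
; It clears its Spline, then uses cosine and sine with RadiusX and RadiusY to add evenly stepped local-space points around the ellipse.
; The same loop spawns a BP_MagneticFieldPoints actor at each computed offset, used directly as a world transform without the magnet's own transform.
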(event EventBeginPlay
  (bind _pointcount (Variables|Default|GetPointCount))
  (bind _spline (Variables|Default|GetSpline))
  (Spline|ClearSplinePoints _spline true)
  (for _index (range 0 (- _pointcount -1))
    (Spline|AddSplinePoint _spline (Math|Vector|MakeVector (* (Math|Trig|Cos(Degrees) (Math|Conversions|ToFloat(Integer) (* _index (/ 360 _pointcount)))) (Variables|Default|GetRadiusX)) (* (Math|Trig|Sin(Degrees) (Math|Conversions|ToFloat(Integer) (* _index (/ 360 _pointcount)))) (Variables|Default|GetRadiusY)) 0.0) "Local" true)
    (Game|SpawnActorfromClass "/Game/Magnet/BP_MagneticFieldPoints.BP_MagneticFieldPoints_C" (Math|Conversions|ToTransform(Vector) (Math|Vector|MakeVector (* (Math|Trig|Cos(Degrees) (Math|Conversions|ToFloat(Integer) (* _index (/ 360 _pointcount)))) (Variables|Default|GetRadiusX)) (* (Math|Trig|Sin(Degrees) (Math|Conversions|ToFloat(Integer) (* _index (/ 360 _pointcount)))) (Variables|Default|GetRadiusY)) 0.0)) "Undefined" "MultiplyWithRoot" 0 0)))

(event Collision|EventActorBeginOverlap
  (params (OtherActor :type Actor%20Object%20Reference)))

(event EventTick
  (params (DeltaSeconds :type Float%20%28single-precision%29)))

(fn ConstructionScript)