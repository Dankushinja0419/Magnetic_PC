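; Magnetic physics object that is pulled toward the player pawn.
; BeginPlay caches player pawn 0 as the target and enables physics simulation on the Cube.
; Each Tick pushes the Cube along the normalized direction from the actor to the target, scaled by ForceStrength regardless of distance.
; When the Sphere overlaps the player, it sets AttachedToPlayer, which stops the pull without performing any attachment.
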(event OnComponentBeginOverlap(Sphere)
  (params (OverlappedComponent :type Primitive%20Component%20Object%20Reference) (OtherActor :type Actor%20Object%20Reference) (OtherComp :type Primitive%20Component%20Object%20Reference) (OtherBodyIndex :type Integer) (bFromSweep :type Boolean) (SweepResult :type Hit%20Result%20Structure%20%28by%20ref%29))
  (if (== OtherActor (Game|Player|GetPlayerPawn 0))
    (Variables|Default|SetAttachedToPlayer true)))

(event EventBeginPlay
  (Variables|Default|SetTargetActor (Game|Player|GetPlayerPawn 0))
  (Physics|SetSimulatePhysics (Variables|Default|GetCube) true))

(event Collision|EventActorBeginOverlap
  (params (OtherActor :type Actor%20Object%20Reference)))

(event EventTick
  (params (DeltaSeconds :type Float%20%28single-precision%29))
  (if (Utilities|IsValid (Variables|Default|GetTargetActor))
    (if (not (Variables|Default|GetAttachedToPlayer))
      (Physics|AddForce (Variables|Default|GetCube) (* (Math|Vector|Normalize (- (Transformation|GetActorLocation (Variables|Default|GetTargetActor)) (Transformation|GetActorLocation))) (Variables|Default|GetForceStrength)) "None" false))))

(fn ConstructionScript)