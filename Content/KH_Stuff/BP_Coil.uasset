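; Magnetic coil actor that boosts the force of every BP_MagneticTarget in the level while the BP_MagneticRod overlaps its capsule.
; On the authority, begin overlap adds a fixed force step to each target and end overlap subtracts it, clamped at zero, so overlapping coils stack.
; At BeginPlay it caches actors and runs DisableCoil, which hides the coil and turns off its collision.
; Unconnected nodes hold an unused BP_MagneticCubes variant.
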(event OnComponentBeginOverlap(Capsule)
  (params (OverlappedComponent :type Primitive%20Component%20Object%20Reference) (OtherActor :type Actor%20Object%20Reference) (OtherComp :type Primitive%20Component%20Object%20Reference) (OtherBodyIndex :type Integer) (bFromSweep :type Boolean) (SweepResult :type Hit%20Result%20Structure%20%28by%20ref%29))
  ;[0.15 0.15 0.15 0.5] Call Events while Collide/Exit Rod Actor
  (CallFunction|AddMagneticForce OtherActor))

(event OnComponentEndOverlap(Capsule)
  (params (OverlappedComponent :type Primitive%20Component%20Object%20Reference) (OtherActor :type Actor%20Object%20Reference) (OtherComp :type Primitive%20Component%20Object%20Reference) (OtherBodyIndex :type Integer))
  ;[0.15 0.15 0.15 0.5] Call Events while Collide/Exit Rod Actor
  (CallFunction|MinusMagneticForce OtherActor))

(event Custom|MinusMagneticForce
  (params (OtherActor :type Actor%20Object%20Reference))
  ;[0.15 0.15 0.15 0.5] Minus Magnetic Force Base On Coil Count
  (if (Ability|HasAuthority)
    (if (== OtherActor (Variables|Default|GetBP_MagneticRod))
      (for _array_element (Variables|Default|GetBP_MagneticTarget)
        (if (< (- (Variables|/Game/KH_Stuff/BP_MagneticTarget.BP_MagneticTarget_C|GetMagneticForce _array_element) 2.75e+04) 0.0)
          (Default|SetMagneticForce _array_element 0.0)
          (else
            (Default|SetMagneticForce _array_element (- (Variables|/Game/KH_Stuff/BP_MagneticTarget.BP_MagneticTarget_C|GetMagneticForce _array_element) 2.75e+04))))))))

(event Custom|DisableCoil
  ;[0.15 0.15 0.15 0.5] Disable Coils
  (Default|SetMagneticForce (Variables|Default|GetBP_MagneticTarget) 0.0)
  (for _array_element (Variables|Default|GetAll%20Coils)
    (Rendering|SetActorHiddenInGame true)
    (Collision|SetActorEnableCollision false)))

(event Custom|AddMagneticForce
  (params (OtherActor :type Actor%20Object%20Reference))
  ;[0.15 0.15 0.15 0.5] Add Magnetic Force Base On Coil Count
  (if (Ability|HasAuthority)
    (if (== OtherActor (Variables|Default|GetBP_MagneticRod))
      (for _array_element (Variables|Default|GetBP_MagneticTarget)
        (Default|SetMagneticForce _array_element (+ (Variables|/Game/KH_Stuff/BP_MagneticTarget.BP_MagneticTarget_C|GetMagneticForce _array_element) 2.75e+04))))))

(event EventBeginPlay
  (bind _outactors (Actor|GetAllActorsOfClass "BP_Coil_C"))
  (Variables|Default|SetAll%20Coils _outactors)
  (CallFunction|DisableCoil)
  (bind _returnvalue (Actor|GetActorOfClass "/Game/KH_Stuff/BP_MagneticRod.BP_MagneticRod_C"))
  (Variables|Default|SetBP_MagneticRod _returnvalue)
  (bind _outactors_2 (Actor|GetAllActorsOfClass "/Game/KH_Stuff/BP_MagneticTarget.BP_MagneticTarget_C"))
  (Variables|Default|SetBP_MagneticTarget _outactors_2))

(event Collision|EventActorBeginOverlap
  (params (OtherActor :type Actor%20Object%20Reference)))

(event EventTick
  (params (DeltaSeconds :type Float%20%28single-precision%29)))

(fn ConstructionScript)