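; BP_MagneticCubes is a physics-simulated cube that gets pulled toward a magnetic source actor.
; Tick pushes the cube toward the source, scaling force by linear distance falloff, with zero force beyond a range derived from force strength.
; SetMagneticForce feeds the same update chain to change strength.
; The logic to stop pulling once attached to the target is unfinished and never runs.
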(event Custom|SetMagneticForce
  (params (MagneticForce :type Float%20%28double-precision%29))
  ;[0.15 0.15 0.15 0.5] Update Magnetic Force Applying To The Cubes (Constantly Trigger with Tick And Change Force By Calling Event)
  (Variables|Default|SetMagneticForce MagneticForce)
  (Variables|Default|SetMaxForceRange (/ (Variables|Default|GetMagneticForce) 5e+02))
  (if (Utilities|IsValid (Variables|Default|GetTargetActor))
    (if (not (Variables|Default|GetAttachedToTarget))
      (CallFunction|CheckForceRecuceOverDistance)
      (Physics|AddForce (Variables|Default|GetCube) (* (Math|Vector|Normalize (- (Transformation|GetActorLocation (Variables|Default|GetTargetActor)) (Transformation|GetWorldLocation (Variables|Default|GetCube)))) (Variables|Default|GetMagneticForce) (Variables|Default|GetMagneticForceDistanceMultiplyer)) "None" false))))

(event Custom|CheckForceRecuceOverDistance
  (bind _targetactor (Variables|Default|GetTargetActor))
  (bind _maxforcerange (Variables|Default|GetMaxForceRange))
  (bind _cube (Variables|Default|GetCube))
  (bind _returnvalue (Transformation|GetActorLocation _targetactor))
  (bind _returnvalue_2 (Transformation|GetWorldLocation _cube))
  (bind _returnvalue_3 (Math|Vector|Distance(Vector) _returnvalue _returnvalue_2))
  ;[0.15 0.15 0.15 0.5] Magnetic Force Reduce Over Distance
  (if (<= _returnvalue_3 _maxforcerange)
    (bind _output_get (Variables|Default|SetMagneticForceDistanceMultiplyer (- 1.0 (/ _returnvalue_3 _maxforcerange))))
    (if (> _output_get 1.0)
      (Variables|Default|SetMagneticForceDistanceMultiplyer 1.0)
      (elif (< _output_get 0.0)
        (bind _output_get_2 (Variables|Default|SetMagneticForceDistanceMultiplyer 0.0))))
    (else
      (Variables|Default|SetMagneticForceDistanceMultiplyer 0.0)))
  (if false
    (Development|PrintString (Utilities|String|ToString(Float) _output_get_2))))

(event Collision|EventActorBeginOverlap
  (params (OtherActor :type Actor%20Object%20Reference)))

(event EventTick
  (params (DeltaSeconds :type Float%20%28single-precision%29))
  ;[0.15 0.15 0.15 0.5] Update Magnetic Force Applying To The Cubes (Constantly Trigger with Tick And Change Force By Calling Event)
  (Variables|Default|SetMagneticForce (stale Custom|SetMagneticForce MagneticForce))
  (Variables|Default|SetMaxForceRange (/ (Variables|Default|GetMagneticForce) 5e+02))
  (if (Utilities|IsValid (Variables|Default|GetTargetActor))
    (if (not (Variables|Default|GetAttachedToTarget))
      (CallFunction|CheckForceRecuceOverDistance)
      (Physics|AddForce (Variables|Default|GetCube) (* (Math|Vector|Normalize (- (Transformation|GetActorLocation (Variables|Default|GetTargetActor)) (Transformation|GetWorldLocation (Variables|Default|GetCube)))) (Variables|Default|GetMagneticForce) (Variables|Default|GetMagneticForceDistanceMultiplyer)) "None" false))))

(event EventBeginPlay
  (Variables|Default|SetTargetActor (Variables|Default|GetMagnetic%20Source))
  (Physics|SetSimulatePhysics (Variables|Default|GetCube) true))

(fn ConstructionScript)

(fn NewFunction)

(fn NewFunction0)