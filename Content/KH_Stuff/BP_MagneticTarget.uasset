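; BP_MagneticTarget is a magnet actor that pulls tagged physics objects toward its root.
; BeginPlay caches actors with the chosen tag.
; Tick and SetMagneticForce share a loop adding force toward the target to each static mesh root component.
; CheckForceRecuceOverDistance fades the pull linearly to zero at a range derived from MagneticForce, printing the multiplier for debugging.
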(event Custom|SetMagneticForce
  (params (MagneticForce :type Float%20%28double-precision%29))
  ;[0.15 0.15 0.15 0.5] Set Magnetic Force Of Taged Static Mesh Towards Target
  (Variables|Default|SetMagneticForce MagneticForce)
  (Variables|Default|SetMaxForceRange (/ (Variables|Default|GetMagneticForce) 1e+02))
  (for _array_element (Variables|Default|GetMagneticObjects)
    (bind _output_get (Variables|Default|SetAllMagneticObjects _array_element))
    (bind _asstatic_mesh_component (Utilities|Casting|CastToStaticMeshComponent (Variables|/Script/Engine.Actor|GetRootComponent _output_get)))
    (CallFunction|CheckForceRecuceOverDistance)
    (Physics|AddForce _asstatic_mesh_component (* (Math|Vector|Normalize (- (Transformation|GetWorldLocation (Variables|Default|GetDefaultSceneRoot)) (Transformation|GetActorLocation (Variables|Default|GetAllMagneticObjects)))) (Variables|Default|GetMagneticForce) (Variables|Default|GetMagneticForceMultiplyer)) "None" false)))

(event Custom|CheckForceRecuceOverDistance
  (bind _maxforcerange (Variables|Default|GetMaxForceRange))
  (bind _defaultsceneroot (Variables|Default|GetDefaultSceneRoot))
  (bind _allmagneticobjects (Variables|Default|GetAllMagneticObjects))
  (bind _returnvalue (Transformation|GetActorLocation _allmagneticobjects))
  (bind _returnvalue_2 (Transformation|GetWorldLocation _defaultsceneroot))
  (bind _returnvalue_3 (Math|Vector|Distance(Vector) _returnvalue_2 _returnvalue))
  ;[0.15 0.15 0.15 0.5] Check Magnetic Force Base On Distance
  (if (<= _returnvalue_3 _maxforcerange)
    (bind _output_get (Variables|Default|SetMagneticForceMultiplyer (- 1.0 (/ _returnvalue_3 _maxforcerange))))
    (if (> _output_get 1.0)
      (Variables|Default|SetMagneticForceMultiplyer 1.0)
      (elif (< _output_get 0.0)
        (bind _output_get_2 (Variables|Default|SetMagneticForceMultiplyer 0.0))))
    (else
      (Variables|Default|SetMagneticForceMultiplyer 0.0)))
  (if true
    (Development|PrintString (Utilities|String|ToString(Float) _output_get_2))))

(event EventBeginPlay
  ;[0.15 0.15 0.15 0.5] Get all actor with Tag
  (bind _outactors (Actor|GetAllActorswithTag (Variables|Default|GetTag)))
  (Variables|Default|SetMagneticObjects _outactors))

(event Collision|EventActorBeginOverlap
  (params (OtherActor :type Actor%20Object%20Reference)))

(event EventTick
  (params (DeltaSeconds :type Float%20%28single-precision%29))
  ;[0.15 0.15 0.15 0.5] Set Magnetic Force Of Taged Static Mesh Towards Target
  (Variables|Default|SetMagneticForce (stale Custom|SetMagneticForce MagneticForce))
  (Variables|Default|SetMaxForceRange (/ (Variables|Default|GetMagneticForce) 1e+02))
  (for _array_element (Variables|Default|GetMagneticObjects)
    (bind _output_get (Variables|Default|SetAllMagneticObjects _array_element))
    (bind _asstatic_mesh_component (Utilities|Casting|CastToStaticMeshComponent (Variables|/Script/Engine.Actor|GetRootComponent _output_get)))
    (CallFunction|CheckForceRecuceOverDistance)
    (Physics|AddForce _asstatic_mesh_component (* (Math|Vector|Normalize (- (Transformation|GetWorldLocation (Variables|Default|GetDefaultSceneRoot)) (Transformation|GetActorLocation (Variables|Default|GetAllMagneticObjects)))) (Variables|Default|GetMagneticForce) (Variables|Default|GetMagneticForceMultiplyer)) "None" false)))

(fn ConstructionScript)